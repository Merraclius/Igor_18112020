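; BaseShell is a projectile Blueprint, apparently the base shell for weapons in a third-person shooter.
; When its Sphere component hits something, it applies point damage to the hit actor, using its forward vector scaled by ImpulsePower as the hit direction.
; It then spawns an impact particle aligned to the surface normal, plays an impact sound at that spot and destroys itself.
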(event OnComponentHit(Sphere)
  (params (HitComponent :type Primitive%20Component%20Object%20Reference) (OtherActor :type Actor%20Object%20Reference) (OtherComp :type Primitive%20Component%20Object%20Reference) (NormalImpulse :type Vector :default "0, 0, 0") (Hit :type Hit%20Result%20Structure%20%28by%20ref%29))
  (bind (_bblockinghit _binitialoverlap _time _distance _location _impactpoint _normal) (Collision|BreakHitResult Hit))
  (Variables|Default|SetHitWorldLocation _location)
  (Game|Damage|ApplyPointDamage OtherActor (Variables|Default|GetDamage) (* (Transformation|GetActorForwardVector) (Variables|Default|GetImpulsePower)) Hit)
  (Effects|SpawnEmitteratLocation (Variables|Default|GetImpactParticle) (Variables|Default|GetHitWorldLocation) (Math|Conversions|RotationFromXVector _normal))
  (Audio|PlaySoundatLocation (Variables|Default|GetImpactSound) (Variables|Default|GetHitWorldLocation) "0, 0, 0" 1.0 1.0 0.0 0 0 0)
  (Actor|DestroyActor))

(fn ConstructionScript)
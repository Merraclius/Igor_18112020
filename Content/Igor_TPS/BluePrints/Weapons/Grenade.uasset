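; Grenade weapon Blueprint, an interactive actor that explodes after a short delay and damages characters.
; Explode disables the interaction zone, light and info display, waits, then plays sound and particles and sets IsExploding.
; It briefly switches DamageZone collision to overlap everything before destroying the actor.
; OnInteractStart extends the parent's interaction logic, applying Damage to the interacting character only while IsExploding is set.
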(event Custom|Explode
  (bind _staticmesh (Variables|Default|GetStaticMesh))
  (bind _returnvalue (Transformation|GetWorldLocation _staticmesh))
  (Collision|SetCollisionProfileName (Variables|Default|GetInteractiveZone) "NoCollision" true :!class /Script/Engine.PrimitiveComponent)
  (Rendering|Components|Light|SetIntensity (Variables|Default|GetPointLight) 0.0)
  (Rendering|SetVisibility (Variables|Default|GetInteractInfo) false false)
  (Utilities|FlowControl|Delay 1.0)
  (Variables|Default|SetIsExploding true)
  (Audio|SpawnSoundatLocation "/Game/StarterContent/Audio/Explosion02.Explosion02" _returnvalue "0, 0, 0" 1.0 1.0 0.0 0 0)
  (Effects|SpawnEmitteratLocation "/Game/Igor_TPS/Particles/P_ky_laser01.P_ky_laser01" _returnvalue)
  (Collision|SetCollisionProfileName (Variables|Default|GetDamageZone) "OverlapAllDynamic" true :!class /Script/Engine.PrimitiveComponent)
  (Utilities|FlowControl|Delay 0.1)
  (Actor|DestroyActor))

(event EventOnInteractStart
  (params (CharacterRef :type Base%20Character%20Object%20Reference))
  (|CallParentFunction CharacterRef)
  (if (Variables|Default|GetIsExploding)
    (Default|ApplyDamage CharacterRef (Variables|Default|GetDamage))))

(fn ConstructionScript
  (|CallParentFunction))
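; BaseWeapon is an interactable weapon actor that the MainCharacter picks up, serving as either a primary gun or a secondary throwable.
; On interaction it hides its prompt and light, then registers with the character through AddWeapon.
; Fire branches on IsSecondary: Shoot plays effects and spawns a shell actor at ShellSpawnPoint.
; Throw spawns a copy of its own class, casts it to Grenade, launches it with a physics impulse and calls Explode.
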(event EventBeginPlay
  (|CallParentFunction)
  (Variables|Default|SetManualInteractive true))

(event EventOnInteract
  (params (CharacterRef :type Base%20Character%20Object%20Reference))
  (|CallParentFunction CharacterRef)
  (bind _asmain_character (Utilities|Casting|CastToMainCharacter CharacterRef))
  (Rendering|SetVisibility (Variables|Default|GetInteractInfo) false false)
  (Development|SetHiddeninGame (Variables|Default|GetPointLight) true false)
  (Default|AddWeapon _asmain_character self (Variables|Default|GetIsSecondary)))

(fn ConstructionScript)

(fn Fire
  (if (Variables|Default|GetIsSecondary)
    (|Throw)
    (else
      (|Shoot))))
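; HealZone is an interactable zone that continuously heals characters while they interact with it.
; Interact start and stop events add characters to a HealTargets list without duplicates and remove them again.
; Each Tick it calls ApplyDamage on every target with negative damage, HealPerSecond scaled by delta time, so healing reuses the damage pipeline.
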(event EventTick
  (params (DeltaSeconds :type Float%20%28single-precision%29))
  (for _array_element (Variables|Default|GetHealTargets)
    (Game|Damage|ApplyDamage _array_element (* -1 (* (Variables|Default|GetHealPerSecond) DeltaSeconds)) 0 0)))

(event EventOnInteractStart
  (params (CharacterRef :type Base%20Character%20Object%20Reference))
  (if (== (Utilities|Array|FindItem (Variables|Default|GetHealTargets) CharacterRef) -1)
    (Utilities|Array|Add (Variables|Default|GetHealTargets) CharacterRef)))

(event EventOnInteractStop
  (params (CharacterRef :type Base%20Character%20Object%20Reference))
  (Utilities|Array|RemoveItem (Variables|Default|GetHealTargets) CharacterRef))

(fn ConstructionScript
  (|CallParentFunction))
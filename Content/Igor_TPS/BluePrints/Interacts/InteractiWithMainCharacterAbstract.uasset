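; Base actor for objects the main character interacts with, showing an InteractPopUp widget for manual interactions.
; BeginPlay fills the widget with the display name and action text, or hides it when the interaction is not manual.
; Interact start and stop events show or hide the prompt message.
; While visible, the widget turns on yaw each tick to face the player pawn.
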(event EventOnInteractStart
  (params (CharacterRef :type Base%20Character%20Object%20Reference))
  (if (Variables|Default|GetManualInteractive)
    (bind _asinteract_pop_up (Utilities|Casting|CastToInteractPopUp (UserInterface|GetUserWidgetObject (Variables|Default|GetInteractInfo))))
    (Default|ShowInteractMessage _asinteract_pop_up)))

(event EventTick
  (params (DeltaSeconds :type Float%20%28single-precision%29))
  (|HandleRotation))

(event EventBeginPlay
  (|PrepareInteractiveInfo))

(event EventOnInteractStop
  (params (CharacterRef :type Base%20Character%20Object%20Reference))
  (if (Variables|Default|GetManualInteractive)
    (bind _asinteract_pop_up (Utilities|Casting|CastToInteractPopUp (UserInterface|GetUserWidgetObject (Variables|Default|GetInteractInfo))))
    (Default|HideInteractMessage _asinteract_pop_up)))

(fn ConstructionScript)
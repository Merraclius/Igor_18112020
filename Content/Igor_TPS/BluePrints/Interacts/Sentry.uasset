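; Sentry turret interactable that turns to face the character interacting with it and fires shotgun shells.
; Interact start stores that character as ActiveTarget and interact stop clears it; each Tick yaws the Scene component toward a valid target's capsule.
; A Delay on Tick paces firing to about once a second, target or not, playing a sound and spawning an explosion effect and 12Gauge actor at ShelSpawnPoint.
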(event EventTick
  (params (DeltaSeconds :type Float%20%28single-precision%29))
  (|FollowActiveTarget)
  (Utilities|FlowControl|Delay 1.0)
  (Audio|PlaySoundatLocation "/Game/Download/FirstPerson/Audio/FirstPersonTemplateWeaponFire02.FirstPersonTemplateWeaponFire02" (Transformation|GetActorLocation) (Transformation|GetActorRotation) 0.5 1.0 0.0 0 0 0)
  (Effects|SpawnEmitteratLocation "/Game/StarterContent/Particles/P_Explosion.P_Explosion" (Transformation|GetWorldLocation (Variables|Default|GetShelSpawnPoint)) (Transformation|GetActorRotation))
  (Game|SpawnActorfromClass "/Game/Igor_TPS/BluePrints/Weapons/12Gauge.12Gauge_C" (Transformation|GetWorldTransform (Variables|Default|GetShelSpawnPoint)) "AlwaysSpawn" 0 0))

(event EventOnInteractStart
  (params (CharacterRef :type Base%20Character%20Object%20Reference))
  (|CallParentFunction CharacterRef)
  (Variables|Default|SetActiveTarget CharacterRef))

(event EventOnInteractStop
  (params (CharacterRef :type Base%20Character%20Object%20Reference))
  (|CallParentFunction CharacterRef)
  (Variables|Default|SetActiveTarget 0))

(fn ConstructionScript
  (|CallParentFunction))
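; Patrol bot interactable whose Sentry travels along a spline and attacks the character that interacts with it.
; Tick plays the FollowPath timeline to move and orient the Sentry until interaction sets ActiveTarget, then stops it until interaction ends.
; While targeting, it turns the Sentry's yaw toward the character and spawns 12Gauge actors with sound and explosion effects, throttled by a Delay.
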(event EventTick
  (params (DeltaSeconds :type Float%20%28single-precision%29))
  (bind _sentry (Variables|Default|GetSentry))
  (if (Utilities|IsValid (Variables|Default|GetActiveTarget))
    (Utilities|FlowControl|Sequence
      (:then_0
        (bind _time (Timeline|FollowPath Stop)
          (:Update
            (Utilities|FlowControl|Sequence
              (:then_0
                (Transformation|SetWorldLocation _sentry (Spline|GetLocationatTime (Variables|Default|GetSpline) _time "World" false) false false))
              (:then_1
                (Transformation|SetWorldRotation _sentry (Math|Conversions|RotationFromXVector (Class|SplineComponent|GetDirectionatTime (Variables|Default|GetSpline) _time "World" false)) false false))))))
      (:then_1
        (|FollowActiveTarget)
        (|FireToActiveTarget)))
    (else
      (Timeline|FollowPath Play))))

(event EventOnInteractStart
  (params (CharacterRef :type Base%20Character%20Object%20Reference))
  (|CallParentFunction CharacterRef)
  (Variables|Default|SetActiveTarget CharacterRef))

(event EventOnInteractStop
  (params (CharacterRef :type Base%20Character%20Object%20Reference))
  (|CallParentFunction CharacterRef)
  (Variables|Default|SetActiveTarget 0))

(fn ConstructionScript
  (|CallParentFunction))
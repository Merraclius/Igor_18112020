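; BaseLamp is a lamp Blueprint whose point light flickers on and off in random colors.
; Tick feeds a randomly timed Delay, which paces each color change and on/off toggle.
; SwitchLight tracks IsLightOn and calls LightOn, which sets a fixed or random intensity, or LightOff, which zeroes it.
; The Tick loop always requests random intensity.
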(event EventBeginPlay
  (|CallParentFunction))

(event EventTick
  (params (DeltaSeconds :type Float%20%28single-precision%29))
  (|CallParentFunction DeltaSeconds)
  (Utilities|FlowControl|Delay (Math|Random|RandomFloatinRange 0.5 2.0))
  (CallFunction|ChangeColor)
  (CallFunction|SwitchLight (not (Variables|Default|GetIsLightOn)) 5e+03 true 2e+03 5e+04))

(fn ConstructionScript)

(fn SwitchLight
  (params (On/Off :type Boolean) (Intensity :type Float%20%28single-precision%29) (IsRandomIntensity :type Boolean) (MinRandomIntensity :type Float%20%28single-precision%29) (MaxRandomIntensity :type Float%20%28single-precision%29))
  (if On/Off
    (CallFunction|Lighton Intensity IsRandomIntensity MinRandomIntensity MaxRandomIntensity)
    (Variables|Default|SetIsLightOn true)
    (else
      (CallFunction|LightOff)
      (Variables|Default|SetIsLightOn false))))

(fn Lighton
  (params (Intensity :type Float%20%28single-precision%29) (IsRandomIntensity :type Boolean) (MinRandomIntensity :type Float%20%28single-precision%29) (MaxRandomIntensity :type Float%20%28single-precision%29))
  (bind _pointlight (Variables|Default|GetPointLight))
  (if IsRandomIntensity
    (Rendering|Components|Light|SetIntensity _pointlight (Math|Random|RandomFloatinRange MinRandomIntensity MaxRandomIntensity))
    (else
      (Rendering|Components|Light|SetIntensity _pointlight Intensity))))

(fn LightOff
  (Rendering|Components|Light|SetIntensity (Variables|Default|GetPointLight) 0.0))

(fn ChangeColor
  (Rendering|Components|Light|SetLightColor (Variables|Default|GetPointLight) (Math|Color|MakeColor (Math|Random|RandomFloat) (Math|Random|RandomFloat) (Math|Random|RandomFloat)) true))
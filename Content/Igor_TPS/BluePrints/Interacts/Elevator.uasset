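; Interactable elevator that carries its platform along a spline, built on a parent interact class.
; Interacting plays the Elevate timeline, which samples the spline by time to set the platform's world location and toggles an at-end flag when finished.
; When interaction stops with that flag set, it waits a second and reverses the timeline from the end.
; Tick hides the interact prompt while the elevator moves.
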(event EventBeginPlay
  (|CallParentFunction) ; This node is disabled and will not be called.\nDrag off pins to build functionality.
)

(event Collision|EventActorBeginOverlap
  (params (OtherActor :type Actor%20Object%20Reference)))

(event EventTick
  (params (DeltaSeconds :type Float%20%28single-precision%29))
  (|CallParentFunction DeltaSeconds)
  (if (Variables|Default|GetElevationInProgress)
    (Rendering|SetVisibility (Variables|Default|GetInteractInfo) false false)))

(event EventOnInteract
  (params (CharacterRef :type Base%20Character%20Object%20Reference))
  (|CallParentFunction CharacterRef)
  (Variables|Default|SetElevationInProgress false)
  (bind _time (Timeline|Elevate Play)
    (:Update
      (Variables|Default|SetElevationInProgress true)
      (Transformation|SetWorldLocation (Variables|Default|GetElevator) (Spline|GetLocationatTime (Variables|Default|GetSpline) _time "World" false) false false))
    (:Finished
      (Variables|Default|SetAtTheEnd (not (Variables|Default|GetAtTheEnd)))
      (Variables|Default|SetElevationInProgress false))))

(event EventOnInteractStop
  (params (CharacterRef :type Base%20Character%20Object%20Reference))
  (|CallParentFunction CharacterRef)
  (if (Variables|Default|GetAtTheEnd)
    (Utilities|FlowControl|Delay 1.0)
    (bind _time (Timeline|Elevate ReverseFromEnd)
      (:Update
        (Variables|Default|SetElevationInProgress true)
        (Transformation|SetWorldLocation (Variables|Default|GetElevator) (Spline|GetLocationatTime (Variables|Default|GetSpline) _time "World" false) false false))
      (:Finished
        (Variables|Default|SetAtTheEnd (not (Variables|Default|GetAtTheEnd)))
        (Variables|Default|SetElevationInProgress false)))))

(fn ConstructionScript
  (|CallParentFunction))
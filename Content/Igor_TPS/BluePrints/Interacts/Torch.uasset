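; Torch is an interactable light Blueprint that adds fire particles and sound to its parent class's light-switching behavior.
; BeginPlay calls SwitchLight with OnOff left unset, while OnInteractStart calls it with OnOff true at a different intensity.
; The SwitchLight override runs the parent logic, matches particle visibility to IsLightOn, and plays an attenuated one-shot fire sound at the actor's location when lit.
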(event EventBeginPlay
  (|CallParentFunction)
  (CallFunction|SwitchLight false 5e+04 false 0.0 1e+04))

(event EventOnInteractStart
  (params (CharacterRef :type Base%20Character%20Object%20Reference))
  (|CallParentFunction CharacterRef)
  (CallFunction|SwitchLight true 1e+04 false 0.0 1e+04))

(event EventTick
  (params (DeltaSeconds :type Float%20%28single-precision%29)))

(fn ConstructionScript
  (|CallParentFunction))

(fn SwitchLight
  (params (On/Off :type Boolean) (Intensity :type Float%20%28single-precision%29) (IsRandomIntensity :type Boolean) (MinRandomIntensity :type Float%20%28single-precision%29) (MaxRandomIntensity :type Float%20%28single-precision%29))
  (bind _islighton (Variables|Default|GetIsLightOn))
  (|CallParentFunction On/Off Intensity IsRandomIntensity MinRandomIntensity MaxRandomIntensity)
  (Rendering|SetVisibility (Variables|Default|GetParticleSystem) _islighton false)
  (if _islighton
    (Audio|PlaySoundatLocation "/Game/Igor_TPS/Audio/Fire01.Fire01" (Transformation|GetActorLocation) "0, 0, 0" 0.7 1.0 0.0 "/Game/Igor_TPS/Audio/TorchFire.TorchFire" 0 0)))
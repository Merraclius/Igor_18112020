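; Platform Blueprint that hovers above world-static surfaces by pushing its physics component upward.
; Each tick it traces straight down from the Platform component over the BounceLength distance.
; On a hit it applies an upward, mass-independent force scaled by BouncePower that grows as the surface gets closer, acting like an undamped spring.
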(event EventBeginPlay
  (|CallParentFunction) ; This node is disabled and will not be called.\nDrag off pins to build functionality.
)

(event Collision|EventActorBeginOverlap
  (params (OtherActor :type Actor%20Object%20Reference)))

(event EventTick
  (params (DeltaSeconds :type Float%20%28single-precision%29))
  (bind _platform (Variables|Default|GetPlatform))
  (bind _returnvalue (Transformation|GetWorldLocation _platform))
  (|CallParentFunction DeltaSeconds)
  (bind (_outhit _returnvalue_2) (Collision|LineTraceForObjects _returnvalue (+ _returnvalue (Math|Vector|MakeVector 0.0 0.0 (* (Math|Float|Absolute(Float) (Variables|Default|GetBounceLength)) -1.0))) (Utilities|Array|MakeArray "ObjectTypeQuery1") false 0 "None"))
  (if _returnvalue_2
    (Physics|AddForce (Variables|Default|GetPlatform) (Math|Vector|MakeVector 0.0 0.0 (* (- 1.0 (.Time (Collision|BreakHitResult _outhit))) (Variables|Default|GetBouncePower))) "None" true)))

(fn ConstructionScript
  (|CallParentFunction))
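; Player character Blueprint for a third-person shooter, handling movement, camera, sprint, interaction and dual-slot weapon use.
; Primary and secondary weapons each have an active slot and an arsenal; newly equipped weapons push the previous one into storage by reattaching it.
; Scroll input re-equips the last stored primary regardless of direction, without removing it from the arsenal.
; Interact messages all tracked interactive actors, and death destroys every held weapon.
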(fn ConstructionScript)

(fn AddWeapon
  (params (Weapon :type Base%20Weapon%20Object%20Reference) (IsSecondary :type Boolean))
  (if IsSecondary
    (CallFunction|SetActiveSecondaryWeapon Weapon)
    (else
      (CallFunction|SetActivePrimaryWeapon Weapon))))

(fn SwitchWeapon
  (params (IsPrevious :type Boolean))
  (bind _arsenal (Variables|Default|GetArsenal))
  (if (!= (Utilities|Array|Length (Variables|Default|GetArsenal)) 0)
    (CallFunction|SetActivePrimaryWeapon (Utilities|Array|Get(acopy) _arsenal (- (Utilities|Array|Length _arsenal) 1)))))

(fn SetActivePrimaryWeapon
  (params (Weapon :type Base%20Weapon%20Object%20Reference))
  (if (Utilities|IsValid (Variables|Default|GetActiveWeapon))
    (Utilities|Array|Add (Variables|Default|GetArsenal) (Variables|Default|GetActiveWeapon))
    (Transformation|AttachComponentToComponent (Variables|Default|GetActiveWeapon) (Variables|Default|GetPrimaryArsenalPlace) "None" "SnapToTarget" "SnapToTarget" "KeepRelative" true))
  (bind _output_get (Variables|Default|SetActiveWeapon Weapon))
  (Transformation|AttachComponentToComponent _output_get (Variables|Default|GetPrimaryActiveWeaponPlace) "None" "SnapToTarget" "SnapToTarget" "KeepRelative" true)
  (Utilities|Array|RemoveItem (Variables|Default|GetManualInteractiveActorRef) (Variables|Default|GetActiveWeapon)))

(fn SetActiveSecondaryWeapon
  (params (Weapon :type Base%20Weapon%20Object%20Reference))
  (if (Utilities|IsValid (Variables|Default|GetSecondaryActiveWeapon))
    (Utilities|Array|Add (Variables|Default|GetSecondaryArsenal) (Variables|Default|GetSecondaryActiveWeapon))
    (Transformation|AttachComponentToComponent (Variables|Default|GetSecondaryActiveWeapon) (Variables|Default|GetSecondaryArsenalPlace) "None" "SnapToTarget" "SnapToTarget" "KeepRelative" true))
  (bind _output_get (Variables|Default|SetSecondaryActiveWeapon Weapon))
  (Transformation|AttachComponentToComponent _output_get (Variables|Default|GetSecondaryActiveWeaponPlace) "None" "SnapToTarget" "SnapToTarget" "KeepRelative" true)
  (Utilities|Array|RemoveItem (Variables|Default|GetManualInteractiveActorRef) (Variables|Default|GetSecondaryActiveWeapon)))

(fn Death
  (|CallParentFunction)
  (Utilities|FlowControl|Sequence
    (:then_0
      (|ClearPrimaryArsenal))
    (:then_1
      (|ClearSecondaryArsenal))
    (:then_2
      (|ClearPrimaryActiveWeapon))
    (:then_3
      (|ClearSecondaryActiveWeapon))))

(event Input|ActionEvents|InputActionInteract
  (params (Key :type Key%20Structure))
  (:Pressed
    (for _array_element (Variables|Default|GetManualInteractiveActorRef)
      (Class|InteractwithMainCharacterIterface|OnInteract(Message) _array_element self))))

(event Input|ActionEvents|InputActionSprint
  (params (Key :type Key%20Structure))
  (bind _charactermovement (Variables|Character|GetCharacterMovement))
  (:Pressed
    (Variables|/Script/Engine.CharacterMovementComponent|SetMaxWalkSpeed _charactermovement 1.2e+03))
  (:Released
    (Variables|/Script/Engine.CharacterMovementComponent|SetMaxWalkSpeed _charactermovement 6e+02)))

(event Input|AxisEvents|InputAxisLookUp
  (params (AxisValue :type Float%20%28single-precision%29))
  (Pawn|Input|AddControllerPitchInput AxisValue))

(event Input|AxisEvents|InputAxisTurn
  (params (AxisValue :type Float%20%28single-precision%29))
  (Pawn|Input|AddControllerYawInput AxisValue))

(event Input|AxisEvents|InputAxisMoveForward
  (params (AxisValue :type Float%20%28single-precision%29))
  (Pawn|Input|AddMovementInput (Transformation|GetActorForwardVector) AxisValue false))

(event Input|AxisEvents|InputAxisMoveRight
  (params (AxisValue :type Float%20%28single-precision%29))
  (Pawn|Input|AddMovementInput (Transformation|GetActorRightVector) AxisValue false))

(event Input|ActionEvents|InputActionScrollUp
  (params (Key :type Key%20Structure))
  (:Pressed
    (CallFunction|SwitchWeapon false)))

(event Input|ActionEvents|InputActionScrollDown
  (params (Key :type Key%20Structure))
  (:Pressed
    (CallFunction|SwitchWeapon true)))

(event Input|ActionEvents|InputActionFire
  (params (Key :type Key%20Structure))
  (:Pressed
    (if (Utilities|IsValid (Variables|Default|GetActiveWeapon))
      (Default|Fire (Variables|Default|GetActiveWeapon)))))

(event Input|ActionEvents|InputActionFireSecondary
  (params (Key :type Key%20Structure))
  (:Pressed
    (if (Utilities|IsValid (Variables|Default|GetSecondaryActiveWeapon))
      (Default|Fire (Variables|Default|GetSecondaryActiveWeapon)))))
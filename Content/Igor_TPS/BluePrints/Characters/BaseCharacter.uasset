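; Base character for a TPS that handles health, damage, death and interaction with overlapped actors.
; AnyDamage and PointDamage both reduce clamped HP, and point damage on a dead character adds an impulse at the hit bone.
; Death ragdolls the mesh, disables movement and capsule collision, resets interaction lists and destroys components under WeaponsPlaces.
; Capsule overlaps send start/stop messages to InteractiWithMainCharacterAbstract actors and track them as manual or automatic interactives.
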(event EventBeginPlay
  (Variables|Default|SetHPCurrent (Variables|Default|GetHPMax)))

(fn ConstructionScript)

(fn ApplyDamage
  (params (Damage :type Float%20%28single-precision%29))
  (bind _output_get (Variables|Default|SetHPCurrent (Math|Float|Clamp(Float) (- (Variables|Default|GetHPCurrent) Damage) 0.0 (Variables|Default|GetHPMax))))
  (if (== _output_get 0.0)
    (CallFunction|Death))
  (return))

(fn Death
  (Variables|Default|SetIsDeath true)
  (Physics|SetSimulatePhysics (Variables|Character|GetMesh) true)
  (Pawn|Components|CharacterMovement|DisableMovement (Variables|Character|GetCharacterMovement))
  (Utilities|FlowControl|Sequence
    (:then_0
      (Variables|Default|SetAutoInteractiveActorRef (Utilities|Array|MakeArray 0)))
    (:then_1
      (Variables|Default|SetManualInteractiveActorRef (Utilities|Array|MakeArray 0)))
    (:then_2
      (Collision|SetCollisionProfileName (Variables|Collision|GetCapsuleComponent) "NoCollision" true :!class /Script/Engine.PrimitiveComponent))
    (:then_3
      (for _array_element (Components|GetChildrenComponents (Variables|Default|GetWeaponsPlaces) true)
        (Components|DestroyComponent _array_element))
      (return))))

(fn ApplyPointDamage
  (params (Damage :type Float%20%28single-precision%29) (HitNormal :type Vector) (BoneName :type Name))
  (CallFunction|ApplyDamage Damage)
  (if (Variables|Default|GetIsDeath)
    (Physics|AddImpulse (Variables|Character|GetMesh) HitNormal BoneName true)
    (Collision|SetCollisionProfileName (Variables|Collision|GetCapsuleComponent) "NoCollision" true :!class /Script/Engine.PrimitiveComponent)))

(fn GetHealthinPercentage
  (return (/ (Variables|Default|GetHPCurrent) (Variables|Default|GetHPMax))))

(event Game|Damage|EventPointDamage
  (params (Damage :type Float%20%28single-precision%29) (DamageType :type Damage%20Type%20Object%20Reference) (HitLocation :type Vector :default "0, 0, 0") (HitNormal :type Vector :default "0, 0, 0") (HitComponent :type Primitive%20Component%20Object%20Reference) (BoneName :type Name :default "None") (ShotFromDirection :type Vector :default "0, 0, 0") (InstigatedBy :type Controller%20Object%20Reference) (DamageCauser :type Actor%20Object%20Reference) (HitInfo :type Hit%20Result%20Structure%20%28by%20ref%29))
  (CallFunction|ApplyPointDamage Damage ShotFromDirection (.HitBoneName (Collision|BreakHitResult HitInfo))))

(event Game|Damage|EventAnyDamage
  (params (Damage :type Float%20%28single-precision%29) (DamageType :type Damage%20Type%20Object%20Reference) (InstigatedBy :type Controller%20Object%20Reference) (DamageCauser :type Actor%20Object%20Reference))
  (CallFunction|ApplyDamage Damage))

(event OnComponentBeginOverlap(CapsuleComponent)
  (params (OverlappedComponent :type Primitive%20Component%20Object%20Reference) (OtherActor :type Actor%20Object%20Reference) (OtherComp :type Primitive%20Component%20Object%20Reference) (OtherBodyIndex :type Integer) (bFromSweep :type Boolean) (SweepResult :type Hit%20Result%20Structure%20%28by%20ref%29))
  (|StartInteraction OtherActor))

(event OnComponentEndOverlap(CapsuleComponent)
  (params (OverlappedComponent :type Primitive%20Component%20Object%20Reference) (OtherActor :type Actor%20Object%20Reference) (OtherComp :type Primitive%20Component%20Object%20Reference) (OtherBodyIndex :type Integer))
  (|StopInteraction OtherActor))
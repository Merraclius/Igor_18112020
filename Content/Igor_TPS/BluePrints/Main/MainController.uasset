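; MainController is the player controller that links the player's character to the main UI widget and manages the start, game and death screens.
; On BeginPlay it creates the widget; StartWithNewCharacter looks up a class by name, spawns it at the "Main" player start and possesses it.
; Tick polls the character to update health and show the death screen once.
; ReloadLevel reopens the current level, while the old interaction-text update is disconnected.
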(event Custom|ReloadLevel
  (bind _returnvalue (Game|GetCurrentLevelName true))
  (Game|OpenLevel(byName) (Utilities|String|StringToName _returnvalue)))

(event Custom|StartWithNewCharacter
  (params (Name :type Name))
  (Variables|Default|SetCharacterDeathIsHandled false)
  (bind _characterclass (CallFunction|GetCharacterClassbyName Name))
  (bind _output_get (Variables|Default|SetMainCharacterClass _characterclass))
  (bind _returnvalue (Game|SpawnActorfromClass _output_get (Transformation|GetActorTransform (Class|GameModeBase|FindPlayerStart (Game|GetGameMode) self "Main")) "Undefined" 0 0))
  (Variables|Default|SetMainCharacterRef _returnvalue)
  (Pawn|UnPossess)
  (Pawn|Possess (Variables|Default|GetMainCharacterRef))
  (Default|ShowGameScreen (Variables|Default|GetMainWindowRef)))

(event EventBeginPlay
  (Utilities|FlowControl|Sequence
    (:then_0
      (bind _returnvalue (UserInterface|CreateWidget "/Game/Igor_TPS/UI/MainWindow.MainWindow_C"))
      (bind _output_get (Variables|Default|SetMainWindowRef _returnvalue))
      (UserInterface|Viewport|AddtoViewport _output_get 0)
      (Default|ShowStartScreen (Variables|Default|GetMainWindowRef)))
    (:then_1
      (bind _asmain_character (Utilities|Casting|CastToMainCharacter (Pawn|GetControlledPawn)))
      (Variables|Default|SetMainCharacterRef _asmain_character))))

(event EventTick
  (params (DeltaSeconds :type Float%20%28single-precision%29))
  (if (Utilities|IsValid (Variables|Default|GetMainCharacterRef))
    (Utilities|FlowControl|Sequence
      (:then_0
        (|UpdateHealthBar))
      (:then_1
        (|HandleDeath)))))

(fn ConstructionScript)

(fn GetCharacterClassbyName
  (params (Name :type Name))
  (return (.Value (Utilities|Map|Find (Variables|Default|GetAvailableCharactersClasses) Name))))